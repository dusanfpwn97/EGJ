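; BP_EnemyGate is a damageable enemy gate that tracks its own health, starting at its maximum on BeginPlay.
; OnHit subtracts damage, prints the remaining HP and pushes it to the health message on its widget component.
; It then plays a sword or arrow impact sound at the gate's location, chosen by damage source.
; GetIsAlive reports whether HP is above zero; the gate has no destruction logic of its own.
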(event `self.ReceiveBeginPlay`
  (set `self.HP` (`self.HPMax`)))

(event `/Game/1_Core/Combat/BP_CombatInterface.OnHit`
  (params (Damage :type "Float (double-precision)") (DamageSource :type "/Game/1_Core/Combat/DamageSource Enum" :default "NewEnumerator0"))
  (bind _output_get (set `self.HP` (- (`self.HP`) Damage)))
  (`KismetSystemLibrary.PrintString` (`KismetStringLibrary.Conv_DoubleToString` _output_get))
  (message `/Game/1_Core/Combat/BP_CombatInterface.UpdateHP` (`WidgetComponent.GetWidget` (`self.Widget`)) (`self.HPMax`) (`self.HP`))
  (`self.Play on Hit Sound` DamageSource))

(fn `GetIsAlive`
  (returns (IsAlive :type Boolean))
  (return (> (`self.HP`) 0.0)))

(fn `Play on Hit Sound`
  (params (NewParam :type "/Game/1_Core/Combat/DamageSource Enum" :default "NewEnumerator0"))
  (bind _returnvalue (`self.K2_GetActorLocation`))
  (switch `/Game/1_Core/Combat/DamageSource` NewParam
    (:`NewEnumerator0`
      (`GameplayStatics.PlaySoundAtLocation` "/Game/3_Sounds/Combat/SC_GateHitSword.SC_GateHitSword" _returnvalue (struct) 1.0 1.0 0.0 null null null null))
    (:`NewEnumerator1`
      (`GameplayStatics.PlaySoundAtLocation` "/Game/3_Sounds/Combat/SC_GateHitArrow.SC_GateHitArrow" _returnvalue (struct) 1.0 1.0 0.0 null null null null))))

(fn `UserConstructionScript`)