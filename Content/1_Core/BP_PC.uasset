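; BP_PC, by its name the player controller, lets the number pad change the game's speed.
; Keys 1 through 9 each set global time dilation to the matching multiplier, so 1 restores normal speed and higher keys speed up the game.
; It has no other logic, as BeginPlay, Tick and the construction script are empty.
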(event `self.ReceiveBeginPlay`)

(event `Key|NumPadOne`
  (params (Key :type "Key Structure"))
  (:`Pressed`
    (`GameplayStatics.SetGlobalTimeDilation` 1.0)))

(event `Key|NumPadTwo`
  (params (Key :type "Key Structure"))
  (:`Pressed`
    (`GameplayStatics.SetGlobalTimeDilation` 2.0)))

(event `Key|NumPadThree`
  (params (Key :type "Key Structure"))
  (:`Pressed`
    (`GameplayStatics.SetGlobalTimeDilation` 3.0)))

(event `Key|NumPadFour`
  (params (Key :type "Key Structure"))
  (:`Pressed`
    (`GameplayStatics.SetGlobalTimeDilation` 4.0)))

(event `Key|NumPadFive`
  (params (Key :type "Key Structure"))
  (:`Pressed`
    (`GameplayStatics.SetGlobalTimeDilation` 5.0)))

(event `Key|NumPadSix`
  (params (Key :type "Key Structure"))
  (:`Pressed`
    (`GameplayStatics.SetGlobalTimeDilation` 6.0)))

(event `Key|NumPadSeven`
  (params (Key :type "Key Structure"))
  (:`Pressed`
    (`GameplayStatics.SetGlobalTimeDilation` 7.0)))

(event `Key|NumPadEight`
  (params (Key :type "Key Structure"))
  (:`Pressed`
    (`GameplayStatics.SetGlobalTimeDilation` 8.0)))

(event `Key|NumPadNine`
  (params (Key :type "Key Structure"))
  (:`Pressed`
    (`GameplayStatics.SetGlobalTimeDilation` 9.0)))

(fn `UserConstructionScript`)