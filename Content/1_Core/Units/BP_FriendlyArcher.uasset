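; BP_FriendlyArcher is a friendly archer unit that shoots pooled arrows at its target.
; BeginPlay pre-spawns BP_ArrowNormal actors high above the origin, and GetAvailableArrow cycles through them round-robin, spawning and adding one when the next is busy.
; OnTargetHit checks that the archer is alive with a valid target in range, then initializes an arrow with unit damage from the Weapon socket and calls UpdateTarget.
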(event `self.ReceiveBeginPlay`
  (`parent.ReceiveBeginPlay`)
  (`self.SpawnArrowPool`))

(event `ShootArrow`
  (bind (_unitinfo_isfriendly _unitinfo_isundead _unitinfo_hp _unitinfo_speed _unitinfo_hpregen _unitinfo_atkspeed _unitinfo_atkrange _unitinfo_damage) (break `UnitInfo` (`self.UnitInfo`)))
  (bind _arrow (`self.GetAvailableArrow`))
  (`/Game/1_Core/Towers/BP_ArrowBase.Init` _arrow _unitinfo_damage (`self.Target`) (`SceneComponent.GetSocketLocation` (`self.Mesh`) "Weapon")))

(event `self.OnTargetHit`
  (bind _isalive (`/Game/1_Core/Combat/BP_CombatInterface.GetIsAlive`))
  (if _isalive
    (bind (_isinrange _success) (`self.IsInRangeOfTarget`))
    (if (and _success _isinrange)
      (bind _newparam (`self.GetTarget`))
      (`/Engine/EditorBlueprintResources/StandardMacros.IsValid` _newparam
        (:`Is Valid`
          (`self.ShootArrow`)
          (`self.UpdateTarget` true))))))

(fn `GetAvailableArrow`
  (returns (Arrow :type "/Game/1_Core/Towers/BP_ArrowBase Object Reference"))
  (locals (NewLocalVar_0 :type "/Game/1_Core/Towers/BP_ArrowNormal Object Reference"))
  (bind _currentarrowindex (`self.CurrentArrowIndex`))
  (bind _arrow_pool_num (`self.Arrow Pool Num`))
  (bind _output (`|GetArrayItem` (`self.ArrowPool`) (`self.CurrentArrowIndex`)))
  (`/Engine/EditorBlueprintResources/StandardMacros.IncrementInt` _currentarrowindex
    (:`  `
      (if (>= _currentarrowindex (`self.Arrow Pool Num`))
        (set `self.CurrentArrowIndex` 0))
      (if (`/Game/1_Core/Towers/BP_ArrowBase.IsAvailable` _output)
        (return _output)
        (else
          ;[1 1 1] If no arrows are available createa new one and add it to the pool
          (bind _returnvalue (`|SpawnActorFromClass` "/Game/1_Core/Towers/BP_ArrowNormal.BP_ArrowNormal_C" (`KismetMathLibrary.MakeTransform` (0.0 0.0 15000.0)) "AlwaysSpawn" "OverrideRootScale" null null))
          (bind _output_get (set `local.NewLocalVar_0` _returnvalue))
          (`KismetArrayLibrary.Array_Add` (`self.ArrowPool`) _output_get)
          (set `/Game/1_Core/Towers/BP_ArrowBase.Index` _arrow_pool_num _returnvalue)
          (set `self.CurrentArrowIndex` _arrow_pool_num)
          (`/Engine/EditorBlueprintResources/StandardMacros.IncrementInt` _arrow_pool_num
            (:`  `
              (return _output_get))))))))

(fn `SpawnArrowPool`
  (for _index (range (`self.Arrow Pool Num`))
    (bind _returnvalue (`|SpawnActorFromClass` "/Game/1_Core/Towers/BP_ArrowNormal.BP_ArrowNormal_C" (`KismetMathLibrary.MakeTransform` (0.0 0.0 15000.0)) "AlwaysSpawn" "OverrideRootScale" null null))
    (set `/Game/1_Core/Towers/BP_ArrowBase.Index` _index _returnvalue)
    (`KismetArrayLibrary.Array_Add` (`self.ArrowPool`) _returnvalue)))

(fn `UserConstructionScript`
  (`parent.UserConstructionScript`))