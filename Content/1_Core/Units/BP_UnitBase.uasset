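; Base battle unit Character that autonomously fights opposing spawner units or marches on gates, with a get-up setup for undead variants.
; A half-second timer picks targets, randomised among the nearest enemies to spread out attackers, while Tick switches between AI movement and combat.
; Timed montage attacks deal damage on hit events, and avoidance groups separate teams.
; Death notifies the spawner, floats the body and spawns a ghost spawner carrying its class.
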(event `self.ReceiveBeginPlay`
  (bind (_unitinfo_isfriendly _unitinfo_isundead _unitinfo_hp) (break `UnitInfo` (`self.UnitInfo`)))
  (set `CharacterMovementComponent.MaxWalkSpeed` (`self.GetSpeed`) (`self.CharacterMovement`))
  (set `self.MaxHP` _unitinfo_hp)
  (`self.SetAvoidanceGroups`)
  (`KismetSystemLibrary.Delay` 0.0)
  (`self.UpdateTarget`)
  ;[1 0 0] rework
  (`KismetSystemLibrary.K2_SetTimer` null "UpdateTarget" 0.5 true))

(event `self.ReceiveTick`
  (params (DeltaSeconds :type "Float (single-precision)"))
  (`self.ControlState`))

(event `OnOpposingUnitSpawned`
  (`self.UpdateTarget`))

(event `SetupForUndead`
  (setmembers `UnitInfo` :`StructRef` (`self.UnitInfo`) :`IsFriendly` false :`IsUndead` true)
  (`CharacterMovementComponent.SetMovementMode` (`self.CharacterMovement`) "MOVE_None" 0)
  (set `self.CachedTargetGate` null)
  (`|PlayMontage` (`self.Mesh`) (`self.GetUpMontage`)
    (:`then`
      (`|ExecutionSequence`
        (:`then_0`
          (`PrimitiveComponent.SetCollisionProfileName` (`self.CapsuleComponent`) "NoCollision" true))
        (:`then_1`
          (bind (_direction _newtrack_0) (`Timeline|Timeline_1` :!via `PlayFromStart`)
            (:`Update`
              (`self.K2_AddActorWorldOffset` (`KismetMathLibrary.MakeVector` 0.0 0.0 (* _newtrack_0 (`GameplayStatics.GetWorldDeltaSeconds`) 40.0))))
            (:`Finished`
              (`PrimitiveComponent.SetCollisionProfileName` (`self.CapsuleComponent`) "Pawn" true)
              (`CharacterMovementComponent.SetMovementMode` (`self.CharacterMovement`) "MOVE_Walking" 0)
              (`self.UpdateTarget`))))))))

(event `StartMoving`
  (if (`self.IsDoingAttackMontage`)
    _
    (elif (`|EnumEquality` (`CharacterMovementComponent.MovementMode` (`self.CharacterMovement`)) "MOVE_Walking")
      (`self.StopCombat`)
      (set `self.IsMoving` true)
      (`|AIMoveTo` self (0.0 0.0 0.0) (`self.Target`) -1.0
        (:`OnSuccess`
          _)
        (:`OnFail`
          _))
      (set `self.IsMoving` false))))

(event `StopMoving`
  (`NavMovementComponent.StopActiveMovement` (`self.CharacterMovement`))
  (`Controller.StopMovement` (`AIBlueprintHelperLibrary.GetAIController` self))
  (set `self.IsMoving` false))

(event `StartCombat`
  (bind (_unitinfo_isfriendly _unitinfo_isundead _unitinfo_hp _unitinfo_speed _unitinfo_hpregen _unitinfo_atkspeed) (break `UnitInfo` (`self.UnitInfo`)))
  (bind _attackmontage (`self.AttackMontage`))
  (if (`|EnumEquality` (`CharacterMovementComponent.MovementMode` (`self.CharacterMovement`)) "MOVE_Walking")
    (`self.StopMoving`)
    (set `self.IsInCombat` true)
    (bind _returnvalue (`KismetSystemLibrary.K2_SetTimerDelegate` (delegate `Attack`) (/ 1.0 _unitinfo_atkspeed)))
    (set `self.CombatTHandle` _returnvalue)
    (bind (_isinrange _success) (`self.IsInRangeOfTarget` :!label _label))
    (if (and _isinrange _success)
      (`|PlayMontage` (`self.Mesh`) _attackmontage
        (:`then`
          (set `self.IsDoingAttackMontage` true)
          ;[1 1 1] Watchdog
          (`KismetSystemLibrary.RetriggerableDelay` (`AnimSequenceBase.SequenceLength` _attackmontage))
          (set `self.IsDoingAttackMontage` false)))
      (else
        (`self.StopCombat`)))))

(event `Attack`
  (`self.UpdateTarget`)
  (goto _label))

(event `StopCombat`
  (set `self.IsInCombat` false)
  (`KismetSystemLibrary.K2_ClearAndInvalidateTimerHandle` (`self.CombatTHandle`)))

(event `OnAttackFinished`
  (set `self.IsDoingAttackMontage` false))

(event `OnTargetHit`
  (bind _isalive (`self.GetIsAlive`))
  (if _isalive
    (bind (_isinrange _success) (`self.IsInRangeOfTarget`))
    (if (and _success _isinrange)
      (bind _newparam (`self.GetTarget`))
      (`/Engine/EditorBlueprintResources/StandardMacros.IsValid` _newparam
        (:`Is Valid`
          (message `/Game/1_Core/Combat/BP_CombatInterface.OnHit` _newparam (`self.GetDamage`))
          (`self.UpdateTarget`))))))

(event `self.OnHit`
  (params (Damage :type "Float (double-precision)"))
  (bind (_maxhp _hp) (`self.GetHP`))
  (bind _isalive (`self.GetIsAlive`))
  (if _isalive
    (setmembers `UnitInfo` :`StructRef` (`self.UnitInfo`) :`HP` (- (`.HP` (`self.GetHP`)) Damage))
    (message `/Game/1_Core/Combat/BP_CombatInterface.UpdateHP` (`WidgetComponent.GetWidget` (`self.Widget`)) _maxhp _hp)
    (if (<= _hp 0.0)
      (`self.Die`))))

(event `Die`
  (bind (_returnvalue_roll _returnvalue_pitch _returnvalue_yaw) (`KismetMathLibrary.BreakRotator` (`self.K2_GetActorRotation`)))
  (bind (_deathlocation_x _deathlocation_y _deathlocation_z) (`KismetMathLibrary.BreakVector` (`self.DeathLocation`)))
  (bind _capsulecomponent (`self.CapsuleComponent`))
  (bind (_unitinfo_isfriendly _unitinfo_isundead) (break `UnitInfo` (`self.UnitInfo`)))
  (if (not _unitinfo_isundead)
    (`/Game/1_Core/Spawner/BP_SpawnerBase.RegisterUnitDied` (`self.Spawner`) self))
  (`self.StopMoving`)
  (`self.StopCombat`)
  (`PrimitiveComponent.SetCollisionEnabled` _capsulecomponent "NoCollision")
  (`PrimitiveComponent.SetCollisionProfileName` _capsulecomponent "NoCollision" false)
  (`|ExecutionSequence`
    (:`then_0`
      (`CharacterMovementComponent.SetAvoidanceEnabled` (`self.CharacterMovement`) false)
      (`ActorComponent.SetComponentTickEnabled` (`self.CharacterMovement`) false)
      (`ActorComponent.SetComponentTickEnabled` (`self.CharacterMovement`) false))
    (:`then_1`
      (set `self.DeathLocation` (`self.K2_GetActorLocation`))
      (`KismetSystemLibrary.Delay` 2.0)
      (bind (_direction _newtrack_0) (`Timeline|Timeline_0` :!via `PlayFromStart`)
        (:`Update`
          (`self.K2_SetActorLocation` (`KismetMathLibrary.MakeVector` _deathlocation_x _deathlocation_y (+ _deathlocation_z _newtrack_0))))
        (:`Finished`
          (`|SpawnActorFromClass` "/Game/1_Core/Spawner/BP_GhostSpawner.BP_GhostSpawner_C" (`KismetMathLibrary.MakeTransform` (`self.K2_GetActorLocation`) (`KismetMathLibrary.MakeRotator` 0.0 0.0 (+ _returnvalue_yaw -90.0))) "Undefined" "OverrideRootScale" null (`GameplayStatics.GetObjectClass` self) null)
          (`self.K2_DestroyActor`))))))

(fn `ControlState`
  (bind _isalive (`self.GetIsAlive`))
  (if _isalive
    (bind (_isinrange _success) (`self.IsInRangeOfTarget`))
    (if _success
      (if _isinrange
        (if (not (`self.IsInCombat`))
          (`self.StartCombat`))
        (elif (not (`self.IsMoving`))
          (`self.StartMoving`))))))

(fn `GetDamage`
  (returns (Damage :type "Float (double-precision)"))
  (bind (_unitinfo_isfriendly _unitinfo_isundead _unitinfo_hp _unitinfo_speed _unitinfo_hpregen _unitinfo_atkspeed _unitinfo_atkrange _unitinfo_damage) (break `UnitInfo` (`self.UnitInfo`)))
  (return _unitinfo_damage))

(fn `GetHP`
  (returns (MaxHP :type "Float (double-precision)") (HP :type "Float (double-precision)"))
  (bind (_unitinfo_isfriendly _unitinfo_isundead _unitinfo_hp) (break `UnitInfo` (`self.UnitInfo`)))
  (return (`self.MaxHP`) _unitinfo_hp))

(fn `GetIsAlive`
  (returns (IsAlive :type Boolean))
  (return (> (`.HP` (`self.GetHP`)) 0.0)))

(fn `GetSpeed`
  (returns (Speed :type "Float (double-precision)"))
  (bind (_unitinfo_isfriendly _unitinfo_isundead _unitinfo_hp _unitinfo_speed) (break `UnitInfo` (`self.UnitInfo`)))
  (return _unitinfo_speed))

(fn `GetTarget`
  (returns (NewParam :type "Actor Object Reference"))
  (bind _target (`self.Target`))
  (bind _isalive (message `/Game/1_Core/Combat/BP_CombatInterface.GetIsAlive` _target))
  (if _isalive
    (return _target)))

(fn `GetTargetWithAliveCheck`
  (returns (NewParam :type "Actor Object Reference"))
  (bind _target (`self.Target`))
  (bind _isalive (message `/Game/1_Core/Combat/BP_CombatInterface.GetIsAlive` _target))
  (if _isalive
    (return _target)
    (else
      (`self.UpdateTarget`)
      (bind _isalive_2 (message `/Game/1_Core/Combat/BP_CombatInterface.GetIsAlive` (`self.Target`)))
      (if _isalive_2
        (return (`self.Target`))
        (else
          (bind _output_get (set `self.Target` null))
          (return _output_get))))))

(fn `IsInRangeOfTarget`
  (returns (IsInRange :type Boolean) (Success :type Boolean))
  (bind (_unitinfo_isfriendly _unitinfo_isundead _unitinfo_hp _unitinfo_speed _unitinfo_hpregen _unitinfo_atkspeed _unitinfo_atkrange) (break `UnitInfo` (`self.UnitInfo`)))
  (bind _newparam (`self.GetTargetWithAliveCheck`))
  (`/Engine/EditorBlueprintResources/StandardMacros.IsValid` _newparam
    (:`Is Valid`
      (return (<= (`self.GetDistanceTo` _newparam self) _unitinfo_atkrange) true))
    (:`Is Not Valid`
      (return false false))))

(fn `SetAvoidanceGroups`
  (bind _charactermovement (`self.CharacterMovement`))
  (bind _unitinfo_isfriendly (break `UnitInfo` (`self.UnitInfo`)))
  (if _unitinfo_isfriendly
    (`CharacterMovementComponent.SetAvoidanceGroupMask` _charactermovement (make `NavAvoidanceMask` true))
    (`CharacterMovementComponent.SetGroupsToAvoidMask` _charactermovement (make `NavAvoidanceMask` true))
    (`CharacterMovementComponent.SetGroupsToIgnoreMask` _charactermovement (make `NavAvoidanceMask` false true))
    (else
      (`CharacterMovementComponent.SetAvoidanceGroupMask` _charactermovement (make `NavAvoidanceMask` false true))
      (`CharacterMovementComponent.SetGroupsToAvoidMask` _charactermovement (make `NavAvoidanceMask` false true))
      (`CharacterMovementComponent.SetGroupsToIgnoreMask` _charactermovement (make `NavAvoidanceMask` true)))))

(fn `UpdateRotation`
  (bind _isalive (`self.GetIsAlive`))
  (if _isalive
    (if (not (`self.IsDoingAttackMontage`))
      (bind _newparam (`self.GetTarget`))
      (`/Engine/EditorBlueprintResources/StandardMacros.IsValid` _newparam))))

(fn `UpdateTarget`
  (locals (DistanceToCurrentTarget :type "Float (double-precision)" :default 0.0))
  (bind _returnvalue (`self.K2_GetActorLocation`))
  (bind (_unitinfo_isfriendly _unitinfo_isundead _unitinfo_hp _unitinfo_speed _unitinfo_hpregen _unitinfo_atkspeed _unitinfo_atkrange) (break `UnitInfo` (`self.UnitInfo`)))
  (bind _target (`self.Target`))
  (bind (_unitinfo_isfriendly_2 _unitinfo_isundead_2) (break `UnitInfo` (`self.UnitInfo`)))
  (bind _spawner (`self.Spawner`))
  (bind (_unitinfo_isfriendly_3 _unitinfo_isundead_3) (break `UnitInfo` (`self.UnitInfo`)))
  (bind _unitinfo_isfriendly_4 (break `UnitInfo` (`self.UnitInfo`)))
  (bind _cachedtargetgate (`self.CachedTargetGate`))
  (bind _opposingspawner (`/Game/1_Core/Spawner/BP_SpawnerBase.GetOpposingSpawner` _spawner))
  (bind _spawnedunits (`/Game/1_Core/Spawner/BP_SpawnerBase.SpawnedUnits` _opposingspawner))
  (bind _returnvalue_2 (`KismetMathLibrary.Clamp` (/ (`KismetArrayLibrary.Array_Length` (`/Game/1_Core/Spawner/BP_SpawnerBase.SpawnedUnits` _spawner)) 2) 1 20))
  (bind _returnvalue_3 (> (`KismetArrayLibrary.Array_Length` _spawnedunits) 0))
  (if (`|EnumEquality` (`CharacterMovementComponent.MovementMode` (`self.CharacterMovement`)) "MOVE_Walking")
    (if _unitinfo_isundead_2
      ;[1 1 1] Get target gate
      ;;[1 1 1] Already figured out which gate is the target. No need to do it again
      (`/Engine/EditorBlueprintResources/StandardMacros.IsValid` _cachedtargetgate :!label _label
        (:`Is Valid`
          (set `self.Target` _cachedtargetgate))
        (:`Is Not Valid`
          (bind _outactors (`GameplayStatics.GetAllActorsOfClass` "/Game/1_Core/BP_Gate.BP_Gate_C"))
          (for _array_element _outactors
            (if _unitinfo_isfriendly_4
              (bind _isuppergate (`/Game/1_Core/BP_Gate.IsUpperGate` _array_element))
              (if (and (not (`/Game/1_Core/BP_Gate.IsFriendly` _array_element)) _isuppergate)
                (bind _output_get (set `self.Target` _array_element :!label _label_2))
                (set `self.CachedTargetGate` _output_get)
                (return))
              (elif (or (and _isuppergate (not _unitinfo_isundead_3)) (and _unitinfo_isundead_3 (not _isuppergate)))
                (goto _label_2))))))
      (else
        (`/Engine/EditorBlueprintResources/StandardMacros.IsValid` _spawner
          (:`Is Valid`
            (`/Engine/EditorBlueprintResources/StandardMacros.IsValid` _opposingspawner
              (:`Is Valid`
                (`/Engine/EditorBlueprintResources/StandardMacros.IsValid` _target
                  (:`Is Valid`
                    (if (`KismetMathLibrary.ClassIsChildOf` (`GameplayStatics.GetObjectClass` _target) "/Game/1_Core/BP_Gate.BP_Gate_C")
                      (if _returnvalue_3
                        (bind (_closestactors _succ) (`/Game/1_Core/Misc/BP_HelperLib.GetClosestAmountOfActors` _spawnedunits _returnvalue_2 _returnvalue :!label _label_3))
                        (if _succ
                          (set `self.Target` (`KismetArrayLibrary.Array_Random` _closestactors))
                          (bind _isinrange (`self.IsInRangeOfTarget` :!label _label_4))
                          (if _isinrange
                            (`self.StartCombat`)
                            (return)
                            (else
                              (`self.StartMoving`)
                              (return)))
                          (else
                            (goto _label))))
                      (else
                        (bind _isalive (message `/Game/1_Core/Combat/BP_CombatInterface.GetIsAlive` _target))
                        (if _isalive
                          (bind _isinrange_2 (`self.IsInRangeOfTarget`))
                          (if _isinrange_2
                            (return)
                            (else
                              (bind (_closestactors_2 _succ_2) (`/Game/1_Core/Misc/BP_HelperLib.GetClosestAmountOfActors` _spawnedunits _returnvalue_2 _returnvalue))
                              (if _succ_2
                                (bind _output (`|GetArrayItem` _closestactors_2))
                                (if (<= (`self.GetDistanceTo` _output self) (* _unitinfo_atkrange 0.95))
                                  (set `self.Target` _output)
                                  (goto _label_4))
                                (else
                                  (goto _label)))))
                          (else
                            (if _returnvalue_3 :!label _label_5
                              (goto _label_3)
                              (else
                                (goto _label))))))))
                  (:`Is Not Valid`
                    (goto _label_5))))
              (:`Is Not Valid`
                (goto _label))))
          (:`Is Not Valid`
            (goto _label)))))))

(fn `UserConstructionScript`)