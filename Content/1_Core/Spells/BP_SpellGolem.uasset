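; BP_SpellGolem is a one-shot spell actor that summons a friendly golem.
; On BeginPlay it finds all BP_FriendlySpawner actors, asks the first one to train a BP_FriendlyGolem through TryToTrainUnit, then destroys itself.
; It holds no other active logic, as the overlap and tick events are disabled.
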(event `self.ReceiveBeginPlay`
  (`parent.ReceiveBeginPlay`)
  (bind _outactors (`GameplayStatics.GetAllActorsOfClass` "/Game/1_Core/Spawner/BP_FriendlySpawner.BP_FriendlySpawner_C"))
  (`/Game/1_Core/Spawner/BP_FriendlySpawner.TryToTrainUnit` (`|GetArrayItem` _outactors) "/Game/1_Core/Units/BP_FriendlyGolem.BP_FriendlyGolem_C")
  (`self.K2_DestroyActor`))

(fn `UserConstructionScript`
  (`parent.UserConstructionScript`))