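; BP_SpellDoom is a Doom spell Blueprint that is unfinished and has no working effect of its own.
; On BeginPlay it calls the parent, then gathers every BP_UnitBase actor and loops over them with an empty body.
; A disconnected chain, which never runs, asks the first BP_FriendlySpawner to train a BP_FriendlyGolem and then destroys the spell actor.
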(event `self.ReceiveBeginPlay`
  (`parent.ReceiveBeginPlay`)
  (bind _outactors (`GameplayStatics.GetAllActorsOfClass` "/Game/1_Core/Units/BP_UnitBase.BP_UnitBase_C"))
  (for _ _outactors
    _))

(fn `UserConstructionScript`
  (`parent.UserConstructionScript`))