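; BP_SpellRepair is a one-shot spell actor that repairs all friendly gates in the level.
; On BeginPlay it runs the parent logic, then finds every BP_FriendlyLowerGate and BP_FriendlyUpperGate actor and calls RepairGate on each.
; It then calls SpendMana and destroys itself, so the whole effect resolves on spawn with no tick or overlap logic.
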(event `self.ReceiveBeginPlay`
  (`parent.ReceiveBeginPlay`)
  (bind _outactors (`GameplayStatics.GetAllActorsOfClass` "/Game/1_Core/Gates/BP_FriendlyLowerGate.BP_FriendlyLowerGate_C"))
  (for _array_element _outactors
    (`/Game/1_Core/Gates/BP_GateBase.RepairGate` _array_element))
  (bind _outactors_2 (`GameplayStatics.GetAllActorsOfClass` "/Game/1_Core/Gates/BP_FriendlyUpperGate.BP_FriendlyUpperGate_C"))
  (for _array_element_2 _outactors_2
    (`/Game/1_Core/Gates/BP_GateBase.RepairGate` _array_element_2))
  (`self.SpendMana`)
  (`self.K2_DestroyActor`))

(fn `UserConstructionScript`
  (`parent.UserConstructionScript`))