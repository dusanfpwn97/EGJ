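; Enemy-side spawner that pairs with the first BP_FriendlySpawner in the level as its opposing spawner on BeginPlay, after the parent's logic.
; A custom event spawns BP_EnemySolider at a random point in the Box, gives it a default controller and adds it to SpawnedUnits.
; StartSpawning is called but empty here, and the two-second looping timer for that event is disconnected, so this graph never triggers spawning.
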(event `self.ReceiveBeginPlay`
  (`parent.ReceiveBeginPlay`)
  (bind _outactors (`GameplayStatics.GetAllActorsOfClass` "/Game/1_Core/Spawner/BP_FriendlySpawner.BP_FriendlySpawner_C"))
  (`self.SetOpposingSpawner` (`|GetArrayItem` _outactors))
  (`self.StartSpawning`))

(event `StartSpawning`)

(event `CustomEvent_0`
  (bind _box (`self.Box`))
  (bind _returnvalue (`|SpawnActorFromClass` "/Game/1_Core/Units/BP_EnemySolider.BP_EnemySolider_C" (`KismetMathLibrary.MakeTransform` (`KismetMathLibrary.RandomPointInBoundingBox` (`SceneComponent.K2_GetComponentLocation` _box) (`BoxComponent.BoxExtent` _box))) "AdjustIfPossibleButAlwaysSpawn" "OverrideRootScale" null self null))
  (`Pawn.SpawnDefaultController` _returnvalue)
  (`KismetArrayLibrary.Array_Add` (`self.SpawnedUnits`) _returnvalue))

(fn `UserConstructionScript`)