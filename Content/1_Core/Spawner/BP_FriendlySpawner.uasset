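; Player-side spawner that trains friendly units for gold, triggered by number keys 1-4 or TryToTrainUnit calls.
; Requests that pass the gold and queue-size checks join a queue mirrored in the HUD bottom bar, with Tick driving its progress bar.
; A timer using each unit's TrainDuration spawns the front unit at a random point inside the box, notifies the opposing enemy spawner, then restarts for the next.
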(event `self.ReceiveBeginPlay`
  (`parent.ReceiveBeginPlay`)
  (bind _outactors (`GameplayStatics.GetAllActorsOfClass` "/Game/1_Core/Spawner/BP_EnemySpawner.BP_EnemySpawner_C"))
  (`self.SetOpposingSpawner` (`|GetArrayItem` _outactors))
  (bind _asbp_hud (cast `/Game/1_Core/UI/Player/BP_HUD` (`PlayerController.GetHUD` (`GameplayStatics.GetPlayerController` 0))))
  (set `self.HUD` _asbp_hud)
  (bind _asbp_pawn (cast `/Game/1_Core/Misc/BP_Pawn` (`GameplayStatics.GetPlayerPawn` 0)))
  (set `self.Pawn` _asbp_pawn))

(event `self.ReceiveTick`
  (params (DeltaSeconds :type "Float (single-precision)"))
  (bind _bottombarref (`/Game/1_Core/UI/Player/BP_HUD.BottomBarRef` (`self.HUD`)))
  (`self.UpdateCooldown` DeltaSeconds)
  (`/Engine/EditorBlueprintResources/StandardMacros.IsValid` (`self.Bottom Bar Ref`)
    (:`Is Not Valid`
      (`/Engine/EditorBlueprintResources/StandardMacros.IsValid` _bottombarref
        (:`Is Valid`
          (set `self.Bottom Bar Ref` _bottombarref))))))

(event `TryToTrainUnit`
  (params (UnitClass :type "/Game/1_Core/Units/BP_UnitBase Class Reference"))
  (bind (_unitinfo _target _ismoving _isincombat _combatthandle _spawner _maxhp _attackmontage _deathmontage _isdoingattackmontage _cachedtargetgate _deathlocation _undeadskeletalmesh _cachedtargetattackpoint _unitimage _trainduration) (defaults `Object` (`|GetArrayItem` (`self.UnitQueue`))))
  (if (`self.CanSpawn` UnitClass)
    (`/Game/1_Core/Misc/BP_Pawn.SpendGold` (`self.Pawn`) (`.BaseGoldCost` (break `UnitInfo` (defaults `Object` UnitClass))))
    (`KismetArrayLibrary.Array_Add` (`self.UnitQueue`) UnitClass)
    (`Widget.SetVisibility` (`/Game/1_Core/UI/Player/WBP_BottomBar.PB_QueueTimer` (`self.Bottom Bar Ref`)) "HitTestInvisible")
    (`/Game/1_Core/UI/Player/WBP_BottomBar.AddUnitToQueue` (`self.Bottom Bar Ref`) UnitClass)
    (if (== (`KismetArrayLibrary.Array_Length` (`self.UnitQueue`)) 1)
      (bind _returnvalue (`KismetSystemLibrary.K2_SetTimerDelegate` (delegate `CustomEvent_0`) _trainduration true :!label _label))
      (set `self.UnieQueueTimer` _returnvalue)
      (bind _output_get (set `self.Cooldown` _trainduration))
      (set `self.QueueTime` _output_get))))

(event `CustomEvent_0`
  (bind _unitqueue (`self.UnitQueue`))
  (bind _box (`self.Box`))
  (bind _pb_queuetimer (`/Game/1_Core/UI/Player/WBP_BottomBar.PB_QueueTimer` (`self.Bottom Bar Ref`)))
  (bind _returnvalue (`|SpawnActorFromClass` (`|GetArrayItem` (`self.UnitQueue`)) (`KismetMathLibrary.MakeTransform` (`KismetMathLibrary.RandomPointInBoundingBox` (`SceneComponent.K2_GetComponentLocation` _box) (`BoxComponent.BoxExtent` _box)) (struct :`Yaw` 90.0)) "AdjustIfPossibleButAlwaysSpawn" "OverrideRootScale" null self null))
  (`|ExecutionSequence`
    (:`then_0`
      (`Pawn.SpawnDefaultController` (`Actor.Instigator` _returnvalue))
      (`KismetArrayLibrary.Array_Add` (`self.SpawnedUnits`) _returnvalue)
      (`self.OnOpposingUnitSpawned` (`self.GetOpposingSpawner`)))
    (:`then_1`
      (`KismetArrayLibrary.Array_Remove` _unitqueue)
      (`PanelWidget.RemoveChildAt` (`/Game/1_Core/UI/Player/WBP_BottomBar.Hbox_UnitQueue` (`self.Bottom Bar Ref`)) 0)
      (if (<= (`KismetArrayLibrary.Array_Length` _unitqueue) 0)
        (`KismetSystemLibrary.K2_ClearAndInvalidateTimerHandle` (`self.UnieQueueTimer`))
        (`ProgressBar.SetPercent` _pb_queuetimer 0.0)
        (`Widget.SetVisibility` _pb_queuetimer "Collapsed")))
    (:`then_2`
      (if (> (`KismetArrayLibrary.Array_Length` (`self.UnitQueue`)) 0)
        (goto _label)))))

(event `Key|One`
  (params (Key :type "Key Structure"))
  (:`Pressed`
    (`self.TryToTrainUnit` "/Game/1_Core/Units/BP_FriendlyPeasant.BP_FriendlyPeasant_C")))

(event `Key|Two`
  (params (Key :type "Key Structure"))
  (:`Pressed`
    (`self.TryToTrainUnit` "/Game/1_Core/Units/BP_FriendlySoldier.BP_FriendlySoldier_C")))

(event `Key|Three`
  (params (Key :type "Key Structure"))
  (:`Pressed`
    (`self.TryToTrainUnit` "/Game/1_Core/Units/BP_FriendlyArcher.BP_FriendlyArcher_C")))

(event `Key|Four`
  (params (Key :type "Key Structure"))
  (:`Pressed`
    (`self.TryToTrainUnit` "/Game/1_Core/Units/BP_FriendlyKnight.BP_FriendlyKnight_C")))

(fn `CanSpawn`
  (params (NewParam :type "/Game/1_Core/Units/BP_UnitBase Class Reference"))
  (returns (CanSpawn :type Boolean))
  (`/Engine/EditorBlueprintResources/StandardMacros.IsValid` (`self.Bottom Bar Ref`)
    (:`Is Valid`
      (if (<= (`KismetArrayLibrary.Array_Length` (`self.UnitQueue`)) 7)
        (if (`self.DoesHaveGoldForUnitSpawn` NewParam)
          (return true)
          (else
            _))))
    (:`Is Not Valid`
      _))
  (return false))

(fn `DoesHaveGoldForUnitSpawn`
  (params (Class :type "/Game/1_Core/Units/BP_UnitBase Class Reference"))
  (returns (NewParam :type Boolean))
  (return (>= (`/Game/1_Core/Misc/BP_Pawn.CurrentGold` (`self.Pawn`)) (`.BaseGoldCost` (break `UnitInfo` (defaults `Object` Class))))))

(fn `UpdateCooldown`
  (params (B :type "Float (double-precision)"))
  (bind _bottom_bar_ref (`self.Bottom Bar Ref`))
  (if (> (`KismetArrayLibrary.Array_Length` (`self.UnitQueue`)) 0)
    (set `self.Cooldown` (- (`self.Cooldown`) B))
    (`/Engine/EditorBlueprintResources/StandardMacros.IsValid` _bottom_bar_ref
      (:`Is Valid`
        (`ProgressBar.SetPercent` (`/Game/1_Core/UI/Player/WBP_BottomBar.PB_QueueTimer` _bottom_bar_ref) (`KismetMathLibrary.MapRangeClamped` (`self.Cooldown`) 0.0 (`self.QueueTime`) 1.0))))))

(fn `UserConstructionScript`)