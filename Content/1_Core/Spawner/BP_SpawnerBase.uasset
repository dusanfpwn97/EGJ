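; BP_SpawnerBase is a base spawner that tracks the units it has spawned and holds a reference to an opposing spawner.
; OnOpposingUnitSpawned forwards the notification to every unit in SpawnedUnits, and RegisterUnitDied removes a dead unit from that list.
; A getter and setter expose the OpposingSpawner link, while the file itself contains no spawning logic.
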(event `OnOpposingUnitSpawned`
  (for _array_element (`self.SpawnedUnits`)
    (`/Game/1_Core/Units/BP_UnitBase.OnOpposingUnitSpawned` _array_element)))

(event `RegisterUnitDied`
  (params (NewParam :type "/Game/1_Core/Units/BP_UnitBase Object Reference"))
  (`KismetArrayLibrary.Array_RemoveItem` (`self.SpawnedUnits`) NewParam))

(fn `GetOpposingSpawner`
  (returns (OpposingSpawner :type "/Game/1_Core/Spawner/BP_SpawnerBase Object Reference"))
  (return (`self.OpposingSpawner`)))

(fn `SetOpposingSpawner`
  (params (Spawner :type "/Game/1_Core/Spawner/BP_SpawnerBase Object Reference"))
  (set `self.OpposingSpawner` Spawner))

(fn `UserConstructionScript`)