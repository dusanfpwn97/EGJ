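; BP_Ghost is a ghost actor whose skeletal mesh travels once along its spline.
; Tick accumulates a progress value at a fixed rate, maps it with a clamp onto spline length, and sets the mesh's world location and rotation from that point, so it holds at the end.
; BeginPlay caches the start transform after a short delay, but only disconnected leftover timeline and rotation experiments read it.
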(event `self.ReceiveBeginPlay`
  (`KismetSystemLibrary.Delay` 0.5)
  (set `self.StartLoc` (`self.K2_GetActorLocation`))
  (set `self.StartRot` (`self.K2_GetActorRotation`)))

(event `self.ReceiveTick`
  (params (DeltaSeconds :type "Float (single-precision)"))
  (bind _spline (`self.Spline`))
  (bind _returnvalue (`KismetMathLibrary.MapRangeClamped` (`self.NewVar_0`) 0.0 1.0 0.0 (`SplineComponent.GetSplineLength` _spline)))
  (set `self.NewVar_0` (+ (`self.NewVar_0`) (* DeltaSeconds 0.2)))
  (`SceneComponent.K2_SetWorldLocation` (`self.SkeletalMesh`) (`SplineComponent.GetLocationAtDistanceAlongSpline` _spline _returnvalue "World") false false)
  (`SceneComponent.K2_SetWorldRotation` (`self.SkeletalMesh`) (`SplineComponent.GetRotationAtDistanceAlongSpline` _spline _returnvalue "World") false false))

(fn `UserConstructionScript`)