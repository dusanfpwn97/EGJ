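; Animated ghost actor that delivers an undead unit: it rises, descends to the ground, then has UndeadSpawner spawn its UnitClass and destroys itself.
; On BeginPlay, a downward trace seeds navmesh point searches with widening radii, accepting only low points and destroying the actor if none qualifies.
; Timelines drive the lift and a rolling descent with randomized sideways waves, alongside pooled appear and landing particles.
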(event `self.ReceiveBeginPlay`
  (bind (_returnvalue_x _returnvalue_y _returnvalue_z) (`KismetMathLibrary.BreakVector` (`self.K2_GetActorLocation`)))
  (bind (_spawnlocation_x _spawnlocation_y _spawnlocation_z) (`KismetMathLibrary.BreakVector` (`self.SpawnLocation`)))
  (bind (_spawnlocation_x_2 _spawnlocation_y_2 _spawnlocation_z_2) (`KismetMathLibrary.BreakVector` (`self.SpawnLocation`)))
  (bind (_startloc_x _startloc_y _startloc_z) (`KismetMathLibrary.BreakVector` (`self.StartLoc`)))
  (bind _newvar_1 (`self.NewVar_1`))
  (bind (_relative_location_x _relative_location_y _relative_location_z) (`KismetMathLibrary.BreakVector` (`self.Relative Location`)))
  (bind (_startloc_x_2 _startloc_y_2) (`KismetMathLibrary.BreakVector` (`self.StartLoc`)))
  (bind _returnvalue (`SceneComponent.K2_GetComponentLocation` (`self.Scene`)))
  (bind _returnvalue_2 (< _spawnlocation_z -600.0))
  (set `self.StartLoc` (`self.K2_GetActorLocation`))
  (set `self.StartRot` (`self.K2_GetActorRotation`))
  (`|ExecutionSequence`
    (:`then_0`
      (bind _outhit (`KismetSystemLibrary.LineTraceSingle` _returnvalue (+ _returnvalue (-700.0 0.0 -3000.0)) "TraceTypeQuery4"))
      (if (`GameplayStatics.BreakHitResult` _outhit)
        (bind (_randomlocation _returnvalue_3) (`NavigationSystemV1.K2_GetRandomLocationInNavigableRadius` (`.ImpactPoint` (`GameplayStatics.BreakHitResult` _outhit)) 100.0 null null))
        (if _returnvalue_3
          (set `self.SpawnLocation` _randomlocation)
          (if _returnvalue_2
            (set `self.Relative Location` (`SceneComponent.RelativeLocation` (`self.SkeletalMesh`)) :!label _label)
            (set `self.Randy` (`KismetMathLibrary.RandomFloatInRange` -600.0 600.0))
            (set `self.Randx` (`KismetMathLibrary.RandomFloatInRange` -600.0 600.0))
            (`|ExecutionSequence`
              (:`then_0`
                ;[1 1 1] Lift the ghost up
                (bind (_direction _newtrack_0) (`Timeline|Timeline_1` :!via `PlayFromStart`)
                  (:`Update`
                    (`self.K2_SetActorLocation` (`KismetMathLibrary.MakeVector` _startloc_x _startloc_y (+ _newtrack_0 _startloc_z))))
                  (:`Finished`
                    ;[1 1 1] Lower the ghost with wavy pattern. Second track in the timeline controls the wave
                    (set `self.UpperZ` _returnvalue_z)
                    (`|ExecutionSequence`
                      (:`then_0`
                        (bind (_direction_2 _newtrack_1 _newtrack_2) (`Timeline|Timeline_2` :!via `PlayFromStart`)
                          (:`Update`
                            (`SceneComponent.K2_SetRelativeRotation` (`self.SkeletalMesh`) (`KismetMathLibrary.MakeRotator` (`KismetMathLibrary.MapRangeUnclamped` _newtrack_1 0.0 1.0 -90.0 300.0)) false false)
                            (`self.K2_SetActorLocation` (`KismetMathLibrary.MakeVector` (+ (`KismetMathLibrary.Lerp` _startloc_x_2 _spawnlocation_x_2 _newtrack_1) (`KismetMathLibrary.MapRangeUnclamped` _newtrack_2 0.0 1.0 0.0 (`self.Randx`))) (+ (`KismetMathLibrary.Lerp` _startloc_y_2 _spawnlocation_y_2 _newtrack_1) (`KismetMathLibrary.MapRangeUnclamped` _newtrack_2 0.0 1.0 0.0 (`self.Randy`))) (`KismetMathLibrary.Lerp` (`self.UpperZ`) (- _spawnlocation_z_2 100.0) _newtrack_1)))
                            ;;[1 0.4635 0.4635] Sketchy centering of the body
                            (`SceneComponent.K2_SetRelativeLocation` (`self.SkeletalMesh`) (`KismetMathLibrary.MakeVector` _relative_location_x (`KismetMathLibrary.Lerp` _relative_location_y (* _newtrack_1 130.0) _newtrack_1) _relative_location_z) false false))
                          (:`Finished`
                            (`KismetSystemLibrary.Delay` 0.5)
                            (`ActorComponent.Deactivate` _newvar_1)
                            (`FXSystemComponent.ReleaseToPool` _newvar_1)
                            (set `self.NewVar_1` null)
                            (`/Game/1_Core/Spawner/UndeadSpawner.Spawn` (`self.UndeadSpawner`) (`self.UnitClass`) (+ (`self.SpawnLocation`) (0.0 0.0 45.0)))
                            (`self.K2_DestroyActor`))))
                      (:`then_1`
                        (`KismetSystemLibrary.Delay` 4.5)
                        (bind _returnvalue_4 (`GameplayStatics.SpawnEmitterAtLocation` "/Game/2_Assets/FX_Ghost23.FX_Ghost23" (`self.SpawnLocation`) (struct) (1.0 1.0 1.0) true "ManualRelease"))
                        (set `self.NewVar_1` _returnvalue_4))))))
              (:`then_1`
                (bind _returnvalue_5 (`GameplayStatics.SpawnEmitterAtLocation` "/Game/2_Assets/FX_GhostAppear.FX_GhostAppear" (`self.StartLoc`) (struct) (1.0 1.0 1.0) true "ManualRelease"))
                (`KismetSystemLibrary.Delay` 0.2)
                (`ActorComponent.Deactivate` _returnvalue_5)))
            (else
              (bind (_randomlocation_2 _returnvalue_6) (`NavigationSystemV1.K2_GetRandomLocationInNavigableRadius` (`.ImpactPoint` (`GameplayStatics.BreakHitResult` _outhit)) 300.0 null "/Script/NavigationSystem.NavigationQueryFilter"))
              (if _returnvalue_6 :!label _label_2
                (set `self.SpawnLocation` _randomlocation_2)
                (if _returnvalue_2
                  (goto _label)
                  (else
                    _)))
              (bind (_randomlocation_3 _returnvalue_7) (`NavigationSystemV1.K2_GetRandomLocationInNavigableRadius` (`.ImpactPoint` (`GameplayStatics.BreakHitResult` _outhit)) 700.0 null null))
              (if _returnvalue_7
                (set `self.SpawnLocation` _randomlocation_3)
                (if _returnvalue_2
                  (goto _label)
                  (else
                    _)))
              (`KismetSystemLibrary.PrintString` "Navigable radius not found! Should not happen generally!" true true (struct :`R` 1.0 :`G` 0.086574 :`A` 1.0) 5.0)
              (`self.K2_DestroyActor`)))
          (else
            (goto _label_2)))))
    (:`then_1`
      (`KismetSystemLibrary.Delay` 0.0)
      (bind _outactors (`GameplayStatics.GetAllActorsOfClass` "/Game/1_Core/Spawner/UndeadSpawner.UndeadSpawner_C"))
      (set `self.UndeadSpawner` (`|GetArrayItem` _outactors)))))

(fn `UserConstructionScript`)