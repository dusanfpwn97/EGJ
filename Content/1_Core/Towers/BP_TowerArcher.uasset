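; BP_TowerArcher is the archer tower Blueprint, adding outline toggling on top of its parent class.
; TurnonOutline and TurnOffOutline switch the custom depth stencil value on the weapon, skeletal and static meshes, presumably to drive a stencil-based outline effect.
; BeginPlay and the construction script only call the parent, while Tick and overlap are disabled stubs, so any other tower behavior comes from the parent.
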(event `self.ReceiveBeginPlay`
  (`parent.ReceiveBeginPlay`))

(event `/Game/1_Core/Misc/BP_InteractionInterface.TurnOnOutline`
  (`PrimitiveComponent.SetCustomDepthStencilValue` (`self.WeaponMesh`) 2)
  (`PrimitiveComponent.SetCustomDepthStencilValue` (`self.SkeletalMesh`) 2)
  (`PrimitiveComponent.SetCustomDepthStencilValue` (`self.StaticMesh`) 2))

(event `/Game/1_Core/Misc/BP_InteractionInterface.TurnOffOutline`
  (`PrimitiveComponent.SetCustomDepthStencilValue` (`self.SkeletalMesh`) 0)
  (`PrimitiveComponent.SetCustomDepthStencilValue` (`self.WeaponMesh`) 0)
  (`PrimitiveComponent.SetCustomDepthStencilValue` (`self.StaticMesh`) 0))

(fn `UserConstructionScript`
  (`parent.UserConstructionScript`))