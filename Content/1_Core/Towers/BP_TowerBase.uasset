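; Base tower Blueprint that targets the nearest spawned unit in range and shoots pooled arrows at it.
; Its Z sign marks it upper or lower, choosing the enemy or undead spawner and the lighting channels.
; A looping timer at attack speed refreshes the target and plays the attack montage, while Tick yaws the mesh.
; ShootArrow draws from a round-robin, growable pool; upgrade component callbacks update stats and restart the timer.
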(event `CustomEvent_0`
  (params (NewParam :type "UpgradesByLevel Structure"))
  (`self.OnUpgrade` NewParam)
  (`self.StartAttacking`))

(event `self.ReceiveBeginPlay`
  (bind (_returnvalue_x _returnvalue_y _returnvalue_z) (`KismetMathLibrary.BreakVector` (`self.K2_GetActorLocation`)))
  (`KismetSystemLibrary.Delay` 0.0)
  (bind _output_get (set `self.IsUpperTower` (not (< _returnvalue_z 0.0))))
  (`self.SetSpawner`)
  (add `/Game/1_Core/Misc/BP_UpgradeComponent.OnUpgraded` (`self.BP_UpgradeComponent`) (delegate `CustomEvent_0`))
  (`/Game/1_Core/Misc/BP_UpgradeComponent.Init` (`self.BP_UpgradeComponent`) self (`self.Widget`) _output_get)
  (`self.SpawnArrowPool`)
  (`self.UpdateTarget`)
  (`KismetSystemLibrary.Delay` (`KismetMathLibrary.RandomFloatInRange` 0.0 0.5))
  (`self.StartAttacking`))

(event `SetSpawner`
  (if (`self.IsUpperTower`)
    (bind _outactors (`GameplayStatics.GetAllActorsOfClass` "/Game/1_Core/Spawner/BP_EnemySpawner.BP_EnemySpawner_C"))
    (set `self.TargetSpawner` (`|GetArrayItem` _outactors))
    (else
      (bind _outactors_2 (`GameplayStatics.GetAllActorsOfClass` "/Game/1_Core/Spawner/UndeadSpawner.UndeadSpawner_C"))
      (set `self.TargetSpawner` (`|GetArrayItem` _outactors_2)))))

(event `StartAttacking`
  (`KismetSystemLibrary.K2_SetTimerDelegate` (delegate `Attack`) (/ 1.0 (`self.AtkSpeed`)) true))

(event `Attack`
  (`self.UpdateTarget`)
  (`/Engine/EditorBlueprintResources/StandardMacros.IsValid` (`self.Target`)
    (:`Is Valid`
      (`|PlayMontage` (`self.SkeletalMesh`) (`self.AttackMontage`) (* (`self.AtkSpeed`) 2.2)))))

(event `ShootArrow`
  (bind _arrow (`self.GetAvailableArrow`))
  (`/Game/1_Core/Towers/BP_ArrowBase.Init` _arrow (`self.Damage`) (`self.Target`) (`SceneComponent.GetSocketLocation` (`self.SkeletalMesh`) "Weapon")))

(event `self.ReceiveTick`
  (params (DeltaSeconds :type "Float (single-precision)"))
  (bind _target (`self.Target`))
  (bind (_returnvalue_roll _returnvalue_pitch _returnvalue_yaw) (`KismetMathLibrary.BreakRotator` (`KismetMathLibrary.FindLookAtRotation` (`self.K2_GetActorLocation`) (`self.K2_GetActorLocation` _target))))
  (`/Engine/EditorBlueprintResources/StandardMacros.IsValid` _target
    (:`Is Valid`
      (`SceneComponent.K2_SetWorldRotation` (`self.SkeletalMesh`) (`KismetMathLibrary.MakeRotator` 0.0 0.0 (- _returnvalue_yaw 90.0)) false false))))

(fn `GetAvailableArrow`
  (returns (Arrow :type "/Game/1_Core/Towers/BP_ArrowBase Object Reference"))
  (locals (NewLocalVar_0 :type "/Game/1_Core/Towers/BP_ArrowNormal Object Reference"))
  (bind _currentarrowindex (`self.CurrentArrowIndex`))
  (bind _arrow_pool_num (`self.Arrow Pool Num`))
  (bind _output (`|GetArrayItem` (`self.ArrowPool`) (`self.CurrentArrowIndex`)))
  (`/Engine/EditorBlueprintResources/StandardMacros.IncrementInt` _currentarrowindex
    (:`  `
      (if (>= _currentarrowindex (`self.Arrow Pool Num`))
        (set `self.CurrentArrowIndex` 0))
      (if (`/Game/1_Core/Towers/BP_ArrowBase.IsAvailable` _output)
        (return _output)
        (else
          ;[1 1 1] If no arrows are available createa new one and add it to the pool
          (bind _returnvalue (`|SpawnActorFromClass` "/Game/1_Core/Towers/BP_ArrowNormal.BP_ArrowNormal_C" (`KismetMathLibrary.MakeTransform` (0.0 0.0 15000.0)) "AlwaysSpawn" "OverrideRootScale" null null))
          (bind _output_get (set `local.NewLocalVar_0` _returnvalue))
          (`KismetArrayLibrary.Array_Add` (`self.ArrowPool`) _output_get)
          (set `/Game/1_Core/Towers/BP_ArrowBase.Index` _arrow_pool_num _returnvalue)
          (set `self.CurrentArrowIndex` _arrow_pool_num)
          (`/Engine/EditorBlueprintResources/StandardMacros.IncrementInt` _arrow_pool_num
            (:`  `
              (return _output_get))))))))

(fn `GetIsAlive`
  (returns (IsAlive :type Boolean))
  (return false))

(fn `IsActorInRange`
  (params (NewParam1 :type "Actor Object Reference"))
  (returns (NewParam :type Boolean))
  (return false))

(fn `OnUpgrade`
  (params (UpgradesByLevel :type "UpgradesByLevel Structure (by ref)"))
  (for _array_element (`.Upgrades` (break `UpgradesByLevel` UpgradesByLevel))
    (switch `EUpgradeType` (`.UpgradeType` (break `IndividualUpgrade` _array_element))
      (:`DAMAGE`
        (set `self.Damage` (`.Value` (break `IndividualUpgrade` _array_element))))
      (:`ATTACK_SPEED`
        (set `self.AtkSpeed` (`.Value` (break `IndividualUpgrade` _array_element))))
      (:`RANGE`
        (set `self.Range` (`.Value` (break `IndividualUpgrade` _array_element))))
      (:`MULTISHOT`
        (`/Engine/EditorBlueprintResources/StandardMacros.IncrementInt` (`self.MultiShotLevel`))))))

(fn `SpawnArrowPool`
  (for _index (range (`self.Arrow Pool Num`))
    (bind _returnvalue (`|SpawnActorFromClass` "/Game/1_Core/Towers/BP_ArrowNormal.BP_ArrowNormal_C" (`KismetMathLibrary.MakeTransform` (0.0 0.0 15000.0)) "AlwaysSpawn" "OverrideRootScale" null null))
    (set `/Game/1_Core/Towers/BP_ArrowBase.Index` _index _returnvalue)
    (`KismetArrayLibrary.Array_Add` (`self.ArrowPool`) _returnvalue)))

(fn `UpdateTarget`
  (bind _target (`self.Target`))
  (bind _spawnedunits (`/Game/1_Core/Spawner/BP_SpawnerBase.SpawnedUnits` (`self.TargetSpawner`)))
  (bind (_distance _returnvalue) (`GameplayStatics.FindNearestActor` (`self.K2_GetActorLocation`) _spawnedunits))
  (`/Engine/EditorBlueprintResources/StandardMacros.IsValid` _target
    (:`Is Valid`
      (bind _isalive (message `/Game/1_Core/Combat/BP_CombatInterface.GetIsAlive` _target))
      (if _isalive
        (return)
        (else
          (if (> (`KismetArrayLibrary.Array_Length` _spawnedunits) 0) :!label _label
            (if (<= _distance (`self.Range`))
              (`/Engine/EditorBlueprintResources/StandardMacros.IsValid` _returnvalue
                (:`Is Valid`
                  (set `self.Target` _returnvalue)
                  (return))
                (:`Is Not Valid`
                  (set `self.Target` null))))
            (else
              (set `self.Target` null))))))
    (:`Is Not Valid`
      (goto _label))))

(fn `UserConstructionScript`
  (bind (_returnvalue_x _returnvalue_y _returnvalue_z) (`KismetMathLibrary.BreakVector` (`self.K2_GetActorLocation`)))
  (bind _returnvalue (< _returnvalue_z 0.0))
  (bind _returnvalue_2 (not _returnvalue))
  (`PrimitiveComponent.SetLightingChannels` (`self.StaticMesh`) _returnvalue_2 _returnvalue _returnvalue_2)
  (`PrimitiveComponent.SetLightingChannels` (`self.SkeletalMesh`) _returnvalue_2 _returnvalue _returnvalue_2)
  (`PrimitiveComponent.SetLightingChannels` (`self.WeaponMesh`) _returnvalue_2 _returnvalue _returnvalue_2))