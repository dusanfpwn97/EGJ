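; BP_ArrowBase is a reusable tower arrow projectile that homes in on a target and deals damage on arrival.
; Init activates it at a start location and scales interpolation rate by target distance, lower when farther.
; Tick lerps it toward the target's current position, facing it, and sends OnHitMessage upon arrival.
; Deinit runs on spawn, hit or lost target, parking the arrow high above, tick disabled and flagged available for pooling.
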(event `self.ReceiveBeginPlay`
  (`self.Deinit`))

(event `self.ReceiveTick`
  (params (DeltaSeconds :type "Float (single-precision)"))
  (bind _target (`self.Target`))
  (bind _returnvalue (`self.K2_GetActorLocation` _target))
  (`/Engine/EditorBlueprintResources/StandardMacros.IsValid` (`self.Target`)
    (:`Is Valid`
      (bind _output_get (set `self.MovementAlpha` (+ (`self.MovementAlpha`) (* DeltaSeconds (`self.ArrowSpeed`)))))
      (if (>= _output_get 1.0)
        (message `/Game/1_Core/Combat/BP_CombatInterface.OnHit` _target (`self.Damage`) "NewEnumerator1")
        (`self.Deinit`)
        (else
          (`self.K2_SetActorLocation` (`KismetMathLibrary.VLerp` (`self.StartLocation`) _returnvalue (`self.MovementAlpha`)))
          (`self.K2_SetActorRotation` (`KismetMathLibrary.Conv_VectorToRotator` (`KismetMathLibrary.Normal` (- _returnvalue (`self.K2_GetActorLocation`))))))))
    (:`Is Not Valid`
      (`self.Deinit`))))

(event `Init`
  (params (Damage :type "Float (double-precision)") (Target :type "Actor Object Reference") (Location :type "Vector Structure"))
  (bind _target (`self.Target`))
  (`self.SetActorTickEnabled` true)
  (set `self.Target` Target)
  (set `self.Damage` Damage)
  (set `self.IsAvailable` false)
  (`self.K2_SetActorLocation` Location)
  (set `self.StartLocation` Location)
  (set `self.MovementAlpha` 0.0)
  (`/Engine/EditorBlueprintResources/StandardMacros.IsValid` _target
    (:`Is Valid`
      (set `self.ArrowSpeed` (`KismetMathLibrary.MapRangeClamped` (`KismetMathLibrary.Vector_Distance` (`self.K2_GetActorLocation` _target) (`self.StartLocation`)) 0.0 1500.0 8.0 2.0)))
    (:`Is Not Valid`
      (set `self.ArrowSpeed` 6.0))))

(event `Deinit`
  (`self.SetActorTickEnabled` false)
  (set `self.Target` null)
  (set `self.Damage` 0.0)
  (`self.K2_SetActorLocation` (0.0 0.0 15000.0))
  (set `self.IsAvailable` true))

(fn `UserConstructionScript`)