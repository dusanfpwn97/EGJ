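; Helper library, apparently a Blueprint function library, with one function that finds a requested number of actors closest to an origin point.
; GetClosestAmountOfActors maps each array index to its distance, then repeatedly takes the minimum value and removes that entry.
; The minimum's position in the values array doubles as actor index and map key.
; It returns the collected actors and a success flag, short-circuiting for empty or single-actor input.
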(fn `GetClosestAmountOfActors`
  (params (Actors :type "Array of Actor Object Reference") (NumOfActors :type Integer) (Origin :type "Vector Structure"))
  (returns (ClosestActors :type "Array of Actor Object Reference") (Succ :type Boolean))
  (locals (Distances :type "Map of Integer to Float (double-precision)") (NewLocalVar_0 :type Integer :default 0) (NewLocalVar_1 :type "Array of Actor Object Reference"))
  (bind _returnvalue (`KismetArrayLibrary.Array_Length` Actors))
  (bind _newlocalvar_1 (`local.NewLocalVar_1`))
  (bind _newlocalvar_1_2 (`local.NewLocalVar_1`))
  (bind _newlocalvar_1_3 (`local.NewLocalVar_1`))
  (bind _newlocalvar_1_4 (`local.NewLocalVar_1`))
  (if (== _returnvalue 0)
    (return _ false)
    (elif (== _returnvalue 1)
      (return (`|MakeArray` (`|GetArrayItem` Actors)) true)
      (else
        (for (_array_element _array_index) Actors
          (`BlueprintMapLibrary.Map_Add` (`local.Distances`) _array_index (`KismetMathLibrary.Vector_Distance` (`Actor.K2_GetActorLocation` _array_element) Origin)))
        (for _ (range NumOfActors)
          (if (> (`BlueprintMapLibrary.Map_Length` (`local.Distances`)) 0)
            (bind _values (`BlueprintMapLibrary.Map_Values` (`local.Distances`)))
            (bind _output_get (set `local.NewLocalVar_0` (`KismetMathLibrary.MinOfFloatArray` _values)))
            (`KismetArrayLibrary.Array_Add` _newlocalvar_1 (`|GetArrayItem` Actors _output_get))
            (if (>= (`KismetArrayLibrary.Array_Length` _newlocalvar_1) NumOfActors)
              (return _newlocalvar_1_3 (> (`KismetArrayLibrary.Array_Length` _newlocalvar_1_3) 0))
              (else
                (`BlueprintMapLibrary.Map_Remove` (`local.Distances`) (`local.NewLocalVar_0`))))
            (else
              (return _newlocalvar_1_4 (> (`KismetArrayLibrary.Array_Length` _newlocalvar_1_4) 0)))))
        (return _newlocalvar_1_2 (> (`KismetArrayLibrary.Array_Length` _newlocalvar_1_2) 0))))))