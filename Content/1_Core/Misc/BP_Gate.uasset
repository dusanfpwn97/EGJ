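; BP_Gate is a damageable gate with a hit point pool and an on-screen health readout.
; HP starts at HPMax on BeginPlay, and OnHit subtracts damage, debug-prints the new value and passes it to the Widget's UpdateHPMessage.
; GetIsAlive reports whether HP is above zero; the gate itself does not clamp HP or react to reaching zero.
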(event `self.ReceiveBeginPlay`
  (set `self.HP` (`self.HPMax`)))

(event `/Game/1_Core/Combat/BP_CombatInterface.OnHit`
  (params (Damage :type "Float (double-precision)"))
  (bind _output_get (set `self.HP` (- (`self.HP`) Damage)))
  (`KismetSystemLibrary.PrintString` (`KismetStringLibrary.Conv_DoubleToString` _output_get))
  (message `/Game/1_Core/Combat/BP_CombatInterface.UpdateHP` (`WidgetComponent.GetWidget` (`self.Widget`)) (`self.HPMax`) (`self.HP`)))

(fn `GetIsAlive`
  (returns (IsAlive :type Boolean))
  (return (> (`self.HP`) 0.0)))

(fn `UserConstructionScript`)