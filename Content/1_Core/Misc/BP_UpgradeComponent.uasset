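; Upgrade component that tracks an owning actor's current level and upgrade data, paired with a tower upgrade widget.
; Init stores the owner and widget component, then hands itself and the owner to the WBP_TowerUpgrade widget.
; Getters expose the full upgrade info or the current level's entry, using levels that count from one.
; Upgrade only increments the level while entries remain and reports success, with no cost check or effect application here.
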(event `Init`
  (params (Owner :type "Actor Object Reference") (WidgetComp :type "WidgetComponent Object Reference"))
  (set `self.OwnerActor` Owner)
  (bind _output_get (set `self.WidgetComp` WidgetComp))
  (bind _aswbp_tower_upgrade (cast `/Game/1_Core/UI/TowerUpgrades/WBP_TowerUpgrade` (`WidgetComponent.GetWidget` _output_get)))
  (`/Game/1_Core/UI/TowerUpgrades/WBP_TowerUpgrade.Init` _aswbp_tower_upgrade self (`self.OwnerActor`)))

(fn `GetCurrentLevelUpgrade`
  (returns (UpgradeByLevel :type "UpgradesByLevel Structure") (Level :type Integer))
  (bind (_upgrades_name _upgrades_description _upgrades_upgradesbylevel) (break `Upgrade` (`self.Upgrades`)))
  (bind _currentlevel (`self.CurrentLevel`))
  (return (`|GetArrayItem` _upgrades_upgradesbylevel (- _currentlevel 1)) _currentlevel))

(fn `GetUpgradeInfo`
  (returns (Upgrade :type "Upgrade Structure"))
  (return (`self.Upgrades`)))

(fn `Upgrade`
  (returns (Succ :type Boolean))
  (bind _currentlevel (`self.CurrentLevel`))
  (bind (_upgrades_name _upgrades_description _upgrades_upgradesbylevel) (break `Upgrade` (`self.Upgrades`)))
  (if (> (`KismetArrayLibrary.Array_Length` _upgrades_upgradesbylevel) _currentlevel)
    (`/Engine/EditorBlueprintResources/StandardMacros.IncrementInt` _currentlevel
      (:`  `
        (return true)))
    (else
      (return false))))