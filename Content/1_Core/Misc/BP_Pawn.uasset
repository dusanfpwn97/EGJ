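; BP_Pawn is a camera pawn that pans along world Y and Z and zooms on a spring arm.
; CamMoveRight and CamMoveUp axis inputs offset the actor, scaled by speed and delta time, with hardcoded border checks and a small dead zone.
; The mouse wheel changes the spring arm length without clamping.
; Tick calls UpdateCameraRotation, which is currently empty.
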(event `self.ReceiveTick`
  (params (DeltaSeconds :type "Float (single-precision)"))
  (`self.UpdateCameraRotation`))

(event `InputAxis|CamMoveRight`
  (params (AxisValue :type "Float (single-precision)"))
  (bind (_returnvalue_x _returnvalue_y) (`KismetMathLibrary.BreakVector` (`self.K2_GetActorLocation`)))
  ;[1 1 1] Camera
  (if (and (> _returnvalue_y -500.0) (< AxisValue -0.1))
    (`self.K2_AddActorWorldOffset` (`KismetMathLibrary.MakeVector` 0.0 (* (`GameplayStatics.GetWorldDeltaSeconds`) (`self.CamRightMoveSpeed`) AxisValue)) :!label _label)
    (elif (and (< _returnvalue_y 2300.0) (> AxisValue 0.1))
      (goto _label))))

(event `InputAxis|CamMoveUp`
  (params (AxisValue :type "Float (single-precision)"))
  (bind (_returnvalue_x _returnvalue_y _returnvalue_z) (`KismetMathLibrary.BreakVector` (`self.K2_GetActorLocation`)))
  ;[1 1 1] Camera
  (if (and (> _returnvalue_z -600.0) (< AxisValue -0.1))
    (`self.K2_AddActorWorldOffset` (`KismetMathLibrary.MakeVector` 0.0 0.0 (* (`GameplayStatics.GetWorldDeltaSeconds`) (`self.CamUpMoveSpeed`) AxisValue)) :!label _label_2)
    (elif (and (< _returnvalue_z 800.0) (> AxisValue 0.1))
      (goto _label_2))))

(event `InputAxisKey|MouseWheelAxis`
  (params (AxisValue :type "Float (single-precision)"))
  (bind _springarm (`self.SpringArm`))
  (set `SpringArmComponent.TargetArmLength` (+ (`SpringArmComponent.TargetArmLength` _springarm) (* AxisValue -50.0)) _springarm))

(fn `UpdateCameraRotation`)

(fn `UserConstructionScript`)